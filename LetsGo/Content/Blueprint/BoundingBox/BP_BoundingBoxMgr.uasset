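; BP_BoundingBoxMgr manages bounding box plane colliders and the monster entry, route and exit points assigned to each.
; Events spawn BoundingBoxPlane actors from a given transform and ID into a /Planes folder and tracked array, or destroy them all.
; SetWallPoint finds the plane by PlaneID, then stores the monster type and point in parallel arrays, replacing entry or exit points and appending route points.
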(event `self.destroyAllPlaneInUE4`
  (bind _planes (`self.planes`))
  (bind _output (`|GetArrayItem` _planes))
  ;[1 1 1] Generate box plane collider
  (while (>= (`KismetArrayLibrary.Array_Length` (`self.planes`)) 1)
    (`self.K2_DestroyActor` _output)
    (`KismetArrayLibrary.Array_RemoveItem` _planes _output)))

(event `self.makePlaneInUE4`
  (params (tr :type "Transform Structure") (id :type Integer))
  ;[1 1 1] Generate box plane collider
  (bind _returnvalue (`|SpawnActorFromClass` "/Game/Blueprint/BoundingBox/BoundingBoxPlane.BoundingBoxPlane_C" tr "Undefined" "OverrideRootScale" null null))
  (`self.SetFolderPath` _returnvalue "/Planes")
  (bind _asbounding_box_plane (cast `/Game/Blueprint/BoundingBox/BoundingBoxPlane` _returnvalue))
  (set `/Game/Blueprint/BoundingBox/BoundingBoxPlane.planeID` id _asbounding_box_plane)
  (`KismetArrayLibrary.Array_Add` (`self.planes`) _returnvalue))

(event `SetWallPoint`
  (params (wallActor :type "Actor Object Reference") (Type :type String) (Point :type "Vector Structure") (MonsterType :type Integer))
  (bind _planepoints (`self.planePoints`))
  ;[1 1 1] 몬스터 생성지점, 없어지는지점, 루트지점 저장
  (for (_array_element _array_index) (`self.planes`)
    (if (== (`/Game/Blueprint/BoundingBox/BoundingBoxPlane.planeID` (cast `/Game/Blueprint/BoundingBox/BoundingBoxPlane` _array_element :!pure true)) (`/Game/Blueprint/BoundingBox/BoundingBoxPlane.planeID` (cast `/Game/Blueprint/BoundingBox/BoundingBoxPlane` wallActor :!pure true)))
      (`KismetArrayLibrary.Array_Set` (`self.planeMonsterType`) _array_index MonsterType)
      (switch `string` Type
        (:`Entry`
          (bind (_entrypoint _routepoint _exitpoint) (break `PlanePoint` (`|GetArrayItem` _planepoints _array_index)))
          (`KismetArrayLibrary.Array_Set` _planepoints _array_index (make `PlanePoint` Point _routepoint _exitpoint)))
        (:`Route`
          (`KismetArrayLibrary.Array_Add` _routepoint Point))
        (:`Exit`
          (`KismetArrayLibrary.Array_Set` _planepoints _array_index (make `PlanePoint` _entrypoint _routepoint Point)))))))

(fn `UserConstructionScript`)