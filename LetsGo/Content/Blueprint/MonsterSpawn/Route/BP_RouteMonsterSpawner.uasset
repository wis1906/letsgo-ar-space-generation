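; BP_RouteMonsterSpawner spawns route-following Monster actors at an entry point on a looping timer once StartSpawn is called.
; Each Monster receives the spawner's speed and route points plus the exit point, then CheckStart is called on it.
; GetRandNum picks an index by MonsterType, random within a range for one type and fixed for the other, selecting mesh, animation Blueprint and scale from parallel arrays.
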(event `StartSpawn`
  (`KismetSystemLibrary.K2_SetTimer` null "SpawnOneTime" 2.5 true))

(event `SpawnOneTime`
  (bind _returnvalue (`|SpawnActorFromClass` "/Game/Blueprint/MonsterSpawn/Route/Monster.Monster_C" (`KismetMathLibrary.MakeTransform` (`self.EntryPoint`) (`self.Rotation`)) "Undefined" "OverrideRootScale" null null))
  (`self.K2_AddActorLocalRotation` _returnvalue (struct :`Pitch` -90.0) false false)
  (bind _asmonster (cast `/Game/Blueprint/MonsterSpawn/Route/Monster` _returnvalue :!pure true))
  (set `/Game/Blueprint/MonsterSpawn/Route/Monster.speed` (`self.MovingSpeed`) _asmonster)
  (bind _output_get (set `/Game/Blueprint/MonsterSpawn/Route/Monster.routePoints` (`self.RoutePoint`) _asmonster))
  (`KismetArrayLibrary.Array_Add` _output_get (`self.ExitPoint`))
  (switch `int` (`self.monsterType`)
    (:`0`
      (set `self.randIdx` (`KismetMathLibrary.RandomIntegerInRange` 0 2))
      (set `self.MovingSpeed` (`self.MovingSpeed`)))
    (:`1`
      (set `self.randIdx` (`KismetMathLibrary.RandomIntegerInRange` 3 3))
      (set `self.MovingSpeed` (`self.MovingSpeed`))))
  (bind _skeletalmesh (`/Game/Blueprint/MonsterSpawn/Route/Monster.SkeletalMesh` _asmonster))
  (`SkinnedMeshComponent.SetSkinnedAssetAndUpdate` _skeletalmesh (`|GetArrayItem` (`self.monsterMeshs`) (`self.randIdx`)) true)
  (`SkeletalMeshComponent.SetAnimInstanceClass` _skeletalmesh (`|GetArrayItem` (`self.monsterAnimBP`) (`self.randIdx`)))
  (`SceneComponent.SetWorldScale3D` _skeletalmesh (`KismetMathLibrary.Conv_DoubleToVector` (`|GetArrayItem` (`self.monsterScales`) (`self.randIdx`))))
  (`/Game/Blueprint/MonsterSpawn/Route/Monster.CheckStart` _asmonster))

(fn `UserConstructionScript`)