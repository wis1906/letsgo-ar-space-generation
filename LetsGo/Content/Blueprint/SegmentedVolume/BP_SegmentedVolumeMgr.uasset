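; Segmented-volume manager that keeps a pool of shadowless plane mesh components, each paired with a two-sided dynamic material.
; BeginPlay pre-fills the pool; popping places a plane hidden at a given transform with its points and visibility flag, growing the pool when empty.
; UpdateItemVisibility always shows the mesh and only stores the passed flag.
; PushAllItem hides active planes and returns them with freshly created materials.
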(event `self.ReceiveBeginPlay`
  (for _ (range 1 (+ (`self.PoolAmounts`) 1))
    (`self.CreateItem`)))

(event `CreateItem`
  (bind _returnvalue (`AddComponent|NODE_AddStaticMeshComponent-0`))
  (`StaticMeshComponent.SetStaticMesh` _returnvalue "/Engine/BasicShapes/Plane.Plane")
  (`PrimitiveComponent.SetCastShadow` _returnvalue false)
  (`SceneComponent.SetVisibility` _returnvalue false false)
  (bind _returnvalue_2 (`PrimitiveComponent.CreateDynamicMaterialInstance` _returnvalue 0 "/Game/Material/Cubemap/DM_TwoSide.DM_TwoSide"))
  (`KismetArrayLibrary.Array_Add` (`self.MeshAndDMPool`) (make `/Game/Blueprint/SegmentedVolume/MeshAndDM` _returnvalue _returnvalue_2 (`|MakeArray` (0.0 0.0 0.0) :!type "Vector Structure"))))

(event `self.popAndInitItem`
  (params (tr :type "Transform Structure") (rects :type "Array of Vector Structure (by ref)") (isVisible :type Boolean))
  (bind _output (`self.PopItem`))
  (bind (_mesh _dm) (break `/Game/Blueprint/SegmentedVolume/MeshAndDM` _output))
  (`SceneComponent.K2_SetWorldTransform` _mesh tr false true)
  (`SceneComponent.SetVisibility` _mesh false false)
  (`KismetArrayLibrary.Array_Add` (`self.UsingItems`) (make `/Game/Blueprint/SegmentedVolume/MeshAndDM` _mesh _dm rects isVisible)))

(event `self.pushAllItem`
  (bind (_mesh _dm _points) (break `/Game/Blueprint/SegmentedVolume/MeshAndDM` (`|GetArrayItem` (`self.UsingItems`))))
  (while (>= (`KismetArrayLibrary.Array_Length` (`self.UsingItems`)) 1)
    (`SceneComponent.SetVisibility` _mesh false false)
    (bind _returnvalue (`PrimitiveComponent.CreateDynamicMaterialInstance` _mesh 0 "/Game/Material/Cubemap/DM_TwoSide.DM_TwoSide"))
    (`KismetArrayLibrary.Array_Add` (`self.MeshAndDMPool`) (make `/Game/Blueprint/SegmentedVolume/MeshAndDM` _mesh _returnvalue _points))
    (`KismetArrayLibrary.Array_Remove` (`self.UsingItems`))))

(event `self.updateItemVisibility`
  (params (idx :type Integer) (isVisible :type Boolean))
  (bind _usingitems (`self.UsingItems`))
  (bind (_mesh _dm _points) (break `/Game/Blueprint/SegmentedVolume/MeshAndDM` (`|GetArrayItem` _usingitems idx)))
  (`SceneComponent.SetVisibility` _mesh true false)
  (`KismetArrayLibrary.Array_Set` _usingitems idx (make `/Game/Blueprint/SegmentedVolume/MeshAndDM` _mesh _dm _points isVisible)))

(fn `PopItem`
  (returns (output :type "/Game/Blueprint/SegmentedVolume/MeshAndDM Structure"))
  (locals (mesh_dm :type "/Game/Blueprint/SegmentedVolume/MeshAndDM Structure"))
  (if (not (> (`KismetArrayLibrary.Array_Length` (`self.MeshAndDMPool`)) 0))
    (`self.CreateItem`))
  (set `local.mesh_dm` (`|GetArrayItem` (`self.MeshAndDMPool`)))
  (`KismetArrayLibrary.Array_Remove` (`self.MeshAndDMPool`))
  (return (`local.mesh_dm`)))

(fn `UserConstructionScript`)