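; SLAM manager Blueprint that visualizes landmarks and camera motion in the world with long-lived debug draws.
; Draw events render landmarks as small points, keyframe cameras as larger points, and frame cameras as a trajectory line chained through PrevCamPos, which InitBPPrevCamPos resets to the origin.
; DrawPoints gates both camera draws but not landmarks, whose outlier-coloring branch is disconnected, so IsOutlier has no effect.
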(event `self.drawLandmark`
  (params (pos :type "Vector Structure") (isOutlier :type Boolean))
  (`KismetSystemLibrary.DrawDebugPoint` pos 2.0 (struct :`R` 1.0 :`G` 1.0 :`A` 1.0) 10000.0))

(event `self.drawKeyframeCamera`
  (params (pos :type "Vector Structure"))
  (if (`self.bDrawPoints`)
    (`KismetSystemLibrary.DrawDebugPoint` pos 10.0 (struct :`G` 0.161335 :`B` 1.0 :`A` 1.0) 10000.0)))

(event `self.drawFrameCamera`
  (params (pos :type "Vector Structure"))
  (if (`self.bDrawPoints`)
    (`KismetSystemLibrary.DrawDebugLine` (`self.prevCamPos`) pos (struct :`G` 0.806797 :`B` 1.0 :`A` 1.0) 10000.0 2.0)
    (set `self.prevCamPos` pos)))

(event `self.initBPPrevCamPos`
  (set `self.prevCamPos` (0.0 0.0 0.0)))

(fn `UserConstructionScript`)